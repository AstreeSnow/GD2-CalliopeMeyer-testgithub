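; BP_Porte is a door that snaps its Modelporte component between closed and open positions.
; Its Activate and Desactivate events both call ToggleOpenClose, which checks the relative X position to pick the other state, printing debug text.
; When BP_ThirdPersonCharacter overlaps the actor, it sends ActivateMessage to each BPControlables element implementing BPI_ControlInterrupteur.
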(event EventBeginPlay)

(event Collision|EventActorBeginOverlap
  (params (OtherActor :type Actor%20Object%20Reference))
  (Utilities|Casting|CastToBP_ThirdPersonCharacter OtherActor)
  (for _array_element (Variables|Default|GetBP_Controlables)
    (if (Utilities|DoesObjectImplementInterface _array_element "/Game/Elements/BPI_ControlInterrupteur.BPI_ControlInterrupteur_C")
      (Class|BPIControlInterrupteur|Activate(Message) _array_element))))

(event EventTick
  (params (DeltaSeconds :type Float%20%28single-precision%29)))

(event EventActivate
  (CallFunction|ToggleOpenClose))

(event EventDesactivate
  (CallFunction|ToggleOpenClose))

(fn ConstructionScript)

(fn ToggleOpenClose
  (if (>= (.x (Variables|/Script/Engine.SceneComponent|GetRelativeLocation (Variables|Default|Getmodelporte))) 1e+01)
    (Development|PrintString "test")
    (Transformation|SetRelativeLocation (Variables|Default|Getmodelporte) "0, 0, 0" false false)
    (else
      (Development|PrintString "Aaaaaah")
      (Transformation|SetRelativeLocation (Variables|Default|Getmodelporte) "100.000000,0.000000,0.000000" false false))))