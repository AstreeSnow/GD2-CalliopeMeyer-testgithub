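; A door Blueprint that opens and closes in response to an external event.
; On BeginPlay it binds its Activation event to an EventLauncher's ActivateControlables dispatcher.
; Each activation toggles the door by snapping the mesh's relative X position between closed and offset, with no interpolation, and prints debug strings.
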(event Custom|Activation
  (CallFunction|ToggleOpenClose))

(event EventBeginPlay
  (EventDispatchers|BindEventtoActivateControlables (Variables|Default|GetEvent%20Launcher) (delegate Custom|Activation)))

(event EventTick
  (params (DeltaSeconds :type Float%20%28single-precision%29)))

(fn ConstructionScript)

(fn ToggleOpenClose
  (if (>= (.x (Variables|/Script/Engine.SceneComponent|GetRelativeLocation (Variables|Default|Getmodelporte))) 1e+01)
    (Development|PrintString "test")
    (Transformation|SetRelativeLocation (Variables|Default|Getmodelporte) "0, 0, 0" false false)
    (else
      (Development|PrintString "Aaaaaah")
      (Transformation|SetRelativeLocation (Variables|Default|Getmodelporte) "100.000000,0.000000,0.000000" false false))))